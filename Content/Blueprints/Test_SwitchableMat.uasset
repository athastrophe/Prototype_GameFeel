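; Test actor that lets the player swap a sphere's material with the E key while standing in a trigger box.
; Box overlaps enable or disable input for player 0 and toggle a text render's visibility.
; Separate looping MultiGates on E alternate two materials on the sphere and two 2D horn sounds; a third MultiGate has nothing connected.
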(event OnComponentBeginOverlap(Box)
  (params (OverlappedComponent :type Primitive%20Component%20Object%20Reference) (OtherActor :type Actor%20Object%20Reference) (OtherComp :type Primitive%20Component%20Object%20Reference) (OtherBodyIndex :type Integer) (bFromSweep :type Boolean) (SweepResult :type Hit%20Result%20Structure%20%28by%20ref%29))
  (Input|EnableInput (Game|GetPlayerController 0))
  (Rendering|ToggleVisibility (Variables|Default|GetTextRender) false))

(event OnComponentEndOverlap(Box)
  (params (OverlappedComponent :type Primitive%20Component%20Object%20Reference) (OtherActor :type Actor%20Object%20Reference) (OtherComp :type Primitive%20Component%20Object%20Reference) (OtherBodyIndex :type Integer))
  (Input|DisableInput (Game|GetPlayerController 0))
  (Rendering|ToggleVisibility (Variables|Default|GetTextRender) false))

(event Input|KeyboardEvents|E
  (params (Key :type Key%20Structure :default "None"))
  (:Pressed
    (Utilities|FlowControl|MultiGate false true -1)))

(event Input|KeyboardEvents|E
  (params (Key :type Key%20Structure :default "None"))
  (bind _sphere_0 (Variables|Default|GetSphere_0))
  (:Pressed
    (Utilities|FlowControl|MultiGate false true -1
      (:Out%200
        (Rendering|Material|SetMaterial _sphere_0 0 "/Engine/MapTemplates/Materials/BasicAsset01.BasicAsset01"))
      (:Out%201
        (Rendering|Material|SetMaterial _sphere_0 0 "/Engine/MapTemplates/Materials/BasicAsset03.BasicAsset03")))))

(event Input|KeyboardEvents|E
  (params (Key :type Key%20Structure :default "None"))
  (:Pressed
    (Utilities|FlowControl|MultiGate false true -1
      (:Out%200
        (Audio|PlaySound2D "/Game/Audio/455602__inspectorj__tripod-horn-blast-single-01.455602__inspectorj__tripod-horn-blast-single-01" 1.0 1.0 0.0 0 0))
      (:Out%201
        (Audio|PlaySound2D "/Game/Audio/27880__stickinthemud__bike-horn-1.27880__stickinthemud__bike-horn-1" 1.0 1.0 0.0 0 0)))))

(fn ConstructionScript)