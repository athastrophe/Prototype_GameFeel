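; Light fixture Blueprint with three spot lights that switch on and off together.
; The ToggleLights event flips the IsOn flag and applies it to the visibility of all three lights.
; The Construction Script applies IsOn to the same lights, so their initial visibility follows that flag.
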(event EventToggleLights
  (bind _output_get (Variables|Default|SetIsOn? (not (Variables|Default|GetIsOn?))))
  (Rendering|SetVisibility (Variables|Default|GetSpotLight1) _output_get false))

(fn ConstructionScript
  (Rendering|SetVisibility (Variables|Default|GetSpotLight1) (Variables|Default|GetIsOn?) false))